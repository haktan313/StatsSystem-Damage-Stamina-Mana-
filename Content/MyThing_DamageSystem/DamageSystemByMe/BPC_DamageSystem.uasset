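; Damage system Blueprint component that tracks current health and the death state for its owner.
; Heal adds to health, clamped between zero and MaxHealth, and returns the new value.
; TakeDamage subtracts the amount from a damage info struct without clamping, then either sets IsDead and calls Death with the death response, or calls DamageResponse with the damage response.
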(event EventBeginPlay)

(event EventTick
  (params (DeltaSeconds :type Float%20%28single-precision%29)))

(fn Heal
  (params (Amount :type Float%20%28double-precision%29))
  (bind _output_get (Variables|Default|SetcurrentHealth (Math|Float|Clamp(Float) (+ Amount (Variables|Default|GetcurrentHealth)) 0.0 (Variables|Default|GetmaxHealth))))
  (return _output_get))

(fn TakeDamage
  (params (aboutDamage :type S%20Damage%20Infoo%20Structure))
  (bind (_amountofdamage _damageresponse _deathresponse) (Utilities|Struct|BreakS_DamageInfoo aboutDamage))
  (bind _output_get (Variables|Default|SetcurrentHealth (- (Variables|Default|GetcurrentHealth) _amountofdamage)))
  (if (<= _output_get 0.0)
    (Variables|Default|SetisDead true)
    (Default|CallDeath _deathresponse)
    (elif true
      (Default|CallDamageResponse _damageresponse))))